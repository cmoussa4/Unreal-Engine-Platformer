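; Moving obstacle actor that kills the player on touch.
; The construction script feeds relative start and end locations and a duration into an InterpToMovement component, intended as a ping-pong path configurable per instance.
; When its sphere component begins overlapping an actor that casts to Player, it calls Death on that player.
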(event `self.Sphere1.OnComponentBeginOverlap`
  (params (OverlappedComponent :type "PrimitiveComponent Object Reference") (OtherActor :type "Actor Object Reference") (OtherComp :type "PrimitiveComponent Object Reference") (OtherBodyIndex :type Integer) (bFromSweep :type Boolean) (SweepResult :type "HitResult Structure (by ref)"))
  (bind _asplayer (cast `/Game/Blueprints/Player` OtherActor))
  (`/Game/Blueprints/Player.Death` _asplayer))

(fn `UserConstructionScript`
  (bind _interptomovement (`self.InterpToMovement`))
  ;[1 1 1] Moving PingPong Movement Function
  (set `InterpToMovementComponent.ControlPoints` (`|MakeArray` (make `InterpControlPoint` (`self.StartLocation`)) (make `InterpControlPoint` (`self.EndLocation`))) _interptomovement)
  (set `InterpToMovementComponent.Duration` (`self.Duration`) _interptomovement))