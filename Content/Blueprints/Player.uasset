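; Player Blueprint for a physics-driven marble that rolls, jumps and dies.
; Horizontal and Vertical axis inputs share one speed-scaled impulse on the Sphere component.
; Releasing Jump applies an upward velocity-change impulse, gated by a CanJump flag that any Hit event resets.
; The Death event sets sphere collision, spawns sparks with an explosion sound, then opens "Level" after a short delay.
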(event `InputAxis|Horizontal`
  (params (AxisValue :type "Float (single-precision)"))
  ;[1 1 1] Marble Movement
  (`PrimitiveComponent.AddImpulse` (`self.Sphere`) (* (`KismetMathLibrary.MakeVector` (stale `InputAxis|Vertical` AxisValue) AxisValue) (`self.Speed`)) "None" false :!label _label))

(event `InputAxis|Vertical`
  (params (AxisValue :type "Float (single-precision)"))
  ;[1 1 1] Marble Movement
  (goto _label))

(event `InputAction|Jump`
  (params (Key :type "Key Structure"))
  ;[1 1 1] Jump Mechanic
  (:`Released`
    (if (`self.CanJump`)
      (`PrimitiveComponent.AddImpulse` (`self.Sphere`) (`KismetMathLibrary.MakeVector` 0.0 0.0 (`self.JumpPower`)) "None" true)
      (set `self.CanJump` false))))

(event `self.ReceiveHit`
  (params (MyComp :type "PrimitiveComponent Object Reference") (Other :type "Actor Object Reference") (OtherComp :type "PrimitiveComponent Object Reference") (bSelfMoved :type Boolean) (HitLocation :type "Vector Structure") (HitNormal :type "Vector Structure") (NormalImpulse :type "Vector Structure") (Hit :type "HitResult Structure (by ref)"))
  ;[1 1 1] Jump Mechanic
  (set `self.CanJump` true))

(event `Death`
  ;[1 1 1] Death Mechanic
  (`PrimitiveComponent.SetCollisionEnabled` (`self.Sphere`) "QueryAndPhysics")
  (`GameplayStatics.SpawnEmitterAtLocation` "/Game/StarterContent/Particles/P_Sparks.P_Sparks" (`SceneComponent.K2_GetComponentLocation` (`self.Sphere`)) (struct) (5.0 5.0 5.0))
  (`GameplayStatics.PlaySound2D` "/Game/StarterContent/Audio/Explosion02.Explosion02" 0.2 1.0 0.0 null null)
  (`KismetSystemLibrary.Delay` 0.5)
  (`GameplayStatics.OpenLevel` "Level"))

(fn `UserConstructionScript`)