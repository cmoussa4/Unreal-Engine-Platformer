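; Coin is a collectible pickup actor that spins in place until the player touches it.
; Tick applies a frame-rate independent local roll rotation scaled by RollSpeed.
; On overlap with a Player, it plays a 2D sound, destroys itself, and calls PointUpdater on the MarbleMode game mode to update points.
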(event `self.ReceiveTick`
  (params (DeltaSeconds :type "Float (single-precision)"))
  ;[1 1 1] Rotate Function
  (`self.K2_AddActorLocalRotation` (* (`KismetMathLibrary.MakeRotator` (`self.RollSpeed`)) DeltaSeconds)))

(event `self.ReceiveActorBeginOverlap`
  (params (OtherActor :type "Actor Object Reference"))
  ;[1 1 1] PickUp Function
  (cast `/Game/Blueprints/Player` OtherActor)
  (`GameplayStatics.PlaySound2D` "/Engine/EditorSounds/Notifications/CompileSuccess.CompileSuccess" 1.0 1.0 0.0 null null)
  (`self.K2_DestroyActor`)
  (bind _asmarble_mode (cast `/Game/Blueprints/MarbleMode` (`GameplayStatics.GetGameMode`)))
  (`/Game/Blueprints/MarbleMode.Point Updater` _asmarble_mode))

(fn `UserConstructionScript`)